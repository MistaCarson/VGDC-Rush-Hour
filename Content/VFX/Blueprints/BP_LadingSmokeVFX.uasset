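; BP_LadingSmokeVFX is a short-lived landing smoke effect actor that activates its LandingSmoke component on BeginPlay and destroys itself after a fixed delay.
; Each tick it slides horizontally along its Velocity without sweeping, ignoring the Z component.
; Horizontal speed decays linearly by rebuilding Velocity from its normalized direction and reduced XY magnitude, with no clamp at zero.
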(event `self.ReceiveBeginPlay`
  (`ActorComponent.Activate` (`self.LandingSmoke`) false)
  (`KismetSystemLibrary.Delay` 3.0)
  (`self.K2_DestroyActor`))

(event `self.ReceiveTick`
  (params (DeltaSeconds :type "Float (single-precision)"))
  (bind (_returnvalue_x _returnvalue_y) (`KismetMathLibrary.BreakVector` (* DeltaSeconds (`self.Velocity`))))
  (`self.K2_SetActorLocation` (+ (`self.K2_GetActorLocation`) (`KismetMathLibrary.MakeVector` _returnvalue_x _returnvalue_y)))
  (bind _output_get (set `self.Magnitude` (`KismetMathLibrary.VSizeXY` (`self.Velocity`))))
  (bind _output_get_2 (set `self.NormalizedVelocity` (`KismetMathLibrary.Normal` (`self.Velocity`))))
  (set `self.Velocity` (* _output_get_2 (- _output_get (* DeltaSeconds 100.0)))))

(fn `UserConstructionScript`)